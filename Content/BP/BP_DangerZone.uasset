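; BP_DangerZone is a danger zone visual that continuously pulses the opacity of its DangerZone component.
; Each Tick adds delta time to a counter and writes an absolute-cosine wave, scaled by fade speed, range and offset, to the materials' Alpha parameter.
; It has no overlap, damage or construction logic, so this graph only drives the visual effect.
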(event EventBeginPlay)

(event Collision|EventActorBeginOverlap
  (params (OtherActor :type Actor%20Object%20Reference)))

(event EventTick
  (params (DeltaSeconds :type Float%20%28single-precision%29))
  (bind _output_get (Variables|Default|SetFadeTimeCount (+ DeltaSeconds (Variables|Default|GetFadeTimeCount))))
  (Rendering|Material|SetScalarParameterValueonMaterials (Variables|Default|GetDangerZone) "Alpha" (+ (* (Math|Float|Absolute(Float) (Math|Trig|Cos(Radians) (* _output_get (Variables|Default|GetFadeSpeed)))) (Variables|Default|GetFadeRange_Const)) (Variables|Default|GetFadeRangeOffset_Const))))

(fn ConstructionScript)