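; BP_Player is a player Blueprint that tests Enhanced Input by printing debug strings.
; BeginPlay enables input for player controller 0 and calls AddMappingContext on its Enhanced Input subsystem, though no mapping context is shown assigned.
; PlayerInputAction prints "Pressed" once per press through a DoOnce, which Completed resets while printing "Released".
; PlayerInputAxis prints its X and Y values; Tick, overlap and the construction script are empty.
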(event Input|EnhancedActionEvents|EnhancedInputActionPlayerInputAction
  (params (ActionValue :type Boolean) (ElapsedSeconds :type Float%20%28double-precision%29) (TriggeredSeconds :type Float%20%28double-precision%29) (InputAction :type Input%20Action%20Object%20Reference :default "/Game/PlayerInputAction.PlayerInputAction"))
  (:Triggered
    (Utilities|FlowControl|DoOnce false :!label _label
      (:Completed
        (Development|PrintString "Pressed"))))
  (:Completed
    (Utilities|FlowControl|Sequence
      (:then_0
        (goto _label Reset))
      (:then_1
        (Development|PrintString "Released")))))

(event Input|EnhancedActionEvents|EnhancedInputActionPlayerInputAxis
  (params (ActionValue :type Vector%202D%20Structure) (ElapsedSeconds :type Float%20%28double-precision%29) (TriggeredSeconds :type Float%20%28double-precision%29) (InputAction :type Input%20Action%20Object%20Reference :default "/Game/PlayerInputAxis.PlayerInputAxis"))
  (bind (_x _y) (Math|Vector2D|BreakVector2D ActionValue))
  (Development|PrintString (Utilities|String|Append "X" (Utilities|String|ToString(Float) _x) "Y" (Utilities|String|ToString(Float) _y))))

(event EventBeginPlay
  (bind _returnvalue (Game|GetPlayerController 0))
  (bind _returnvalue_2 (PlayerController|LocalPlayerSubsystems|GetEnhancedInputLocalPlayerSubsystem _returnvalue))
  (Utilities|FlowControl|Sequence
    (:then_0
      (Input|EnableInput _returnvalue))
    (:then_1
      (Utilities|IsValid _returnvalue_2
        (:Is%20Valid
          (Input|AddMappingContext _returnvalue_2 0 0 "(bIgnoreAllPressedKeysUntilRelease=True,bForceImmediately=False,bNotifyUserSettings=False)"))))))

(event Collision|EventActorBeginOverlap
  (params (OtherActor :type Actor%20Object%20Reference)))

(event EventTick
  (params (DeltaSeconds :type Float%20%28single-precision%29)))

(fn ConstructionScript)