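; BP_MenuHUD is a HUD Blueprint in TestLevel that owns a menu widget and shows or hides it.
; On BeginPlay it creates BP_TestMenuWidget, stores it as Menu, collapses it and adds it to the viewport.
; The DispPause_Event event takes an IsMenu flag and switches the existing widget between Visible and Collapsed, printing debug strings without pausing the game itself.
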(event Custom|DispPause_Event
  (params (IsMenu :type Boolean))
  (if IsMenu
    (Utilities|FlowControl|Sequence
      (:then_0
        (bind _menu (Variables|Default|GetMenu)
          (:then
            (Widget|SetVisibility _menu "Visible")
            (Development|PrintString "Visibility"))
          (:else))))
    (else
      (bind _menu_2 (Variables|Default|GetMenu)
        (:then
          (Widget|SetVisibility _menu_2 "Collapsed")
          (Development|PrintString "Collapsed"))
        (:else)))))

(event EventBeginPlay
  (bind _returnvalue (UserInterface|CreateWidget "/Game/TestLevel/BP/BP_TestMenuWidget.BP_TestMenuWidget_C"))
  (bind _output_get (Variables|Default|SetMenu _returnvalue))
  (Widget|SetVisibility _output_get "Collapsed")
  (UserInterface|Viewport|AddtoViewport _output_get 0)
  (Development|PrintString "Start HUD"))

(event Collision|EventActorBeginOverlap
  (params (OtherActor :type Actor%20Object%20Reference)))

(event EventTick
  (params (DeltaSeconds :type Float%20%28single-precision%29)))

(fn ConstructionScript)