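; BP_PlayerHP is a test-level Blueprint that triggers a player HP action from Enhanced Input.
; BeginPlay adds the InputManager mapping context to player 0's input subsystem, and IA_Decision calls OnHP when its value equals 1.0; OnHP's body is not in this graph.
; A disconnected chain that would create, display and store the BP_TestHP widget, then print its name, never runs.
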(event Input|EnhancedActionEvents|EnhancedInputActionIA_Decision
  (params (ActionValue :type Float%20%28double-precision%29) (ElapsedSeconds :type Float%20%28double-precision%29) (TriggeredSeconds :type Float%20%28double-precision%29) (InputAction :type Input%20Action%20Object%20Reference :default "/Game/TestLevel/KonnoTestLevel/IA_Decision.IA_Decision"))
  (if (== ActionValue 1.0)
    (Class|PlayerHP|OnHP)))

(event EventBeginPlay
  (bind _returnvalue (Game|GetPlayerController 0))
  (bind _returnvalue_2 (PlayerController|LocalPlayerSubsystems|GetEnhancedInputLocalPlayerSubsystem _returnvalue))
  (Utilities|IsValid _returnvalue_2
    (:Is%20Valid
      (Input|AddMappingContext _returnvalue_2 "/Game/TestLevel/KonnoTestLevel/InputManager.InputManager" 0 "(bIgnoreAllPressedKeysUntilRelease=True,bForceImmediately=False,bNotifyUserSettings=False)"))))

(event Collision|EventActorBeginOverlap
  (params (OtherActor :type Actor%20Object%20Reference)))

(event EventTick
  (params (DeltaSeconds :type Float%20%28single-precision%29)))

(fn ConstructionScript)